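; Player character Blueprint for the MMO, handling health, death, attacks and a camera-facing nameplate.
; Damage lowers Health, and death prints a message and sets a lifespan; X requests an Attack on the target through ActionComponent.
; JoinOrCreate joins the most populated non-full, non-empty session, else CreateSession hosts MMOMap as a listen server.
; The automatic JoinOrCreate call, mob tracking and visibility toggles are disconnected.
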(event Custom|TickNameplate
  (params (DeltaSeconds :type Float%20%28single-precision%29))
  (Transformation|SetWorldRotation (Variables|Default|GetNameplateWidgetComponent) (Math|Rotator|FindLookatRotation (Transformation|GetWorldLocation (Variables|Default|GetNameplateWidgetComponent)) (Transformation|GetWorldLocation (Variables|/Script/Engine.PlayerCameraManager|GetTransformComponent (Variables|/Script/Engine.PlayerController|GetPlayerCameraManager (Game|GetPlayerController 0))))) false false))

(event Custom|CreateSession
  (bind _sessionstate (Class|AdvancedSessionsLibrary|GetSessionState))
  (switch Utilities|FlowControl|Switch|SwitchonEBPOnlineSessionState _sessionstate
    (:NoSession
      _)
    (:Creating
      _)
    (:Pending
      _)
    (:Starting
      _)
    (:Ending
      _)
    (:Ended
      _)
    (:Destroying
      _))
  (|DestroySession (Game|GetPlayerController 0)
    (:OnSuccess
      (Development|PrintString "Destroy Session Success"))
    (:OnFailure
      (Development|PrintString "Destroy Session Failure")))
  (|AdvancedSession 0 (Game|GetPlayerController 0) 100 0 false true false true true false false false true
    (:OnSuccess
      (Development|PrintString "Created Session Success")
      (Game|OpenLevel(byName) "MMOMap" true "listen"))
    (:OnFailure
      (Development|PrintString "Created Session Failure"))))

(event Custom|JoinOrCreate
  (|DestroySession (Game|GetPlayerController 0)
    (:OnSuccess
      _)
    (:OnFailure
      _))
  (bind _results (|FindSessionsAdvanced (Game|GetPlayerController 0) 20 false "AllServers" 0 false false false)
    (:OnSuccess
      (Development|PrintString "Found Sessions Success")
      (if (> (Utilities|Array|Length _results) 0)
        (Utilities|Time|ClearandInvalidateTimerbyHandle (Variables|Default|GetJoinSessionTimer))
        (bind (_session _bgotsession) (CallFunction|GetMostPopulatedNonEmptySession _results))
        (if _bgotsession
          (|JoinSession (Game|GetPlayerController 0) _session
            (:OnSuccess
              (Development|PrintString "Join Session Success"))
            (:OnFailure
              (Development|PrintString "Join Session Failure")))
          (else
            (CallFunction|CreateSession :!label _label)))
        (else
          (goto _label))))
    (:OnFailure
      (Development|PrintString "Found Session Failure")
      (goto _label))))

(event Custom|OnDeath
  (Actor|SetLifeSpan 1e+01)
  (Development|PrintString (Utilities|String|Append (Utilities|GetDisplayName self) " has died")))

(event EventBeginPlay
  (|CallParentFunction))

(event Collision|EventActorBeginOverlap
  (params (OtherActor :type Actor%20Object%20Reference)))

(event EventTick
  (params (DeltaSeconds :type Float%20%28single-precision%29))
  (CallFunction|TickNameplate DeltaSeconds)
  (|CallParentFunction DeltaSeconds))

(event EventOnTargeted
  (params (EventInstigator :type Player%20Controller%20Object%20Reference) (TargetedBy :type Actor%20Object%20Reference))
  (|CallParentFunction EventInstigator TargetedBy))

(event EventOnStoppedTargeting
  (params (EventInstigator :type Player%20Controller%20Object%20Reference) (TargetedBy :type Actor%20Object%20Reference))
  (|CallParentFunction EventInstigator TargetedBy))

(event Game|Damage|EventAnyDamage
  (params (Damage :type Float%20%28single-precision%29) (DamageType :type Damage%20Type%20Object%20Reference) (InstigatedBy :type Controller%20Object%20Reference) (DamageCauser :type Actor%20Object%20Reference))
  (Variables|Default|SetHealth (Math|Float|Max(Float) (- (Variables|Default|GetHealth) Damage) 0.0))
  (Class|MMOCharacter|OnHealthChanged))

(event EventOnHealthChanged
  (|CallParentFunction)
  (if (Class|MMOCharacter|IsDead)
    (CallFunction|OnDeath)))

(event Input|KeyboardEvents|X
  (params (Key :type Key%20Structure :default "None"))
  (:Pressed
    (Class|MMOActionComponent|RequestDoAction (Variables|Default|GetActionComponent) "Attack" (Variables|Default|GetTargetActor) "0, 0, 0")))

(fn ConstructionScript)

(fn GetMostPopulatedNonEmptySession
  (params (SessionArray :type Array%20of%20Blueprint%20Session%20Result%20Structures))
  (for _array_element SessionArray
    (if (< (Class|FindSessionsCallbackProxy|GetCurrentPlayers _array_element) (Class|FindSessionsCallbackProxy|GetMaxPlayers _array_element))
      (if (> (Class|FindSessionsCallbackProxy|GetCurrentPlayers _array_element) (LocalVariables|GetLocalMaxPlayers))
        (LocalVariables|SetLocalMaxPlayers (Class|FindSessionsCallbackProxy|GetCurrentPlayers _array_element))
        (LocalVariables|SetLocalSession _array_element)
        (LocalVariables|SetLocalGotSession true))))
  (return (LocalVariables|GetLocalSession) (LocalVariables|GetLocalGotSession)))