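; MMO player controller that handles the death-to-spirit cycle and online session join-or-host logic.
; ReleaseSpirit clears the character's target and hands it to the first valid shrine; ReturnToLife revives the spirit's corpse, both routing clients through server events.
; JoinOrCreate destroys any session, then joins the fullest non-empty session with free slots, falling back to CreateSession to host MMOMap as a listen server.
; Its automatic session-state trigger is disconnected.
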(event Custom|ServerReleaseSpirit
  (CallFunction|ReleaseSpirit))

(event Custom|CreateSession
  (bind _sessionstate (Class|AdvancedSessionsLibrary|GetSessionState))
  (switch Utilities|FlowControl|Switch|SwitchonEBPOnlineSessionState _sessionstate
    (:NoSession
      _)
    (:Creating
      _)
    (:Pending
      _)
    (:Starting
      _)
    (:Ending
      _)
    (:Ended
      _)
    (:Destroying
      _))
  (|DestroySession (Game|GetPlayerController 0)
    (:OnSuccess
      (Development|PrintString "Destroy Session Success"))
    (:OnFailure
      (Development|PrintString "Destroy Session Failure")))
  (|AdvancedSession 0 (Game|GetPlayerController 0) 100 0 false true false true true false false false true
    (:OnSuccess
      (Development|PrintString "Created Session Success")
      (Game|OpenLevel(byName) "MMOMap" true "listen"))
    (:OnFailure
      (Development|PrintString "Created Session Failure"))))

(event Custom|JoinOrCreate
  (|DestroySession (Game|GetPlayerController 0)
    (:OnSuccess
      _)
    (:OnFailure
      _))
  (bind _results (|FindSessionsAdvanced (Game|GetPlayerController 0) 20 false "AllServers" 0 false false false)
    (:OnSuccess
      (Development|PrintString "Found Sessions Success")
      (if (> (Utilities|Array|Length _results) 0)
        (Utilities|Time|ClearandInvalidateTimerbyHandle (Variables|Default|GetJoinSessionTimer))
        (bind (_session _bgotsession) (CallFunction|GetMostPopulatedNonEmptySession _results))
        (if _bgotsession
          (|JoinSession (Game|GetPlayerController 0) _session
            (:OnSuccess
              (Development|PrintString "Join Session Success"))
            (:OnFailure
              (Development|PrintString "Join Session Failure")))
          (else
            (CallFunction|CreateSession :!label _label)))
        (else
          (goto _label))))
    (:OnFailure
      (Development|PrintString "Found Session Failure")
      (goto _label))))

(event Custom|ServerReturnToLife
  (CallFunction|ReturntoLife))

(event EventBeginPlay
  (|CallParentFunction)
  (Development|PrintString (Utilities|GetDisplayName (Pawn|GetControlledPawn))))

(event EventTick
  (params (DeltaSeconds :type Float%20%28single-precision%29)))

(fn ConstructionScript)

(fn GetMostPopulatedNonEmptySession
  (params (Array :type Array%20of%20Blueprint%20Session%20Result%20Structures))
  (for _array_element Array
    (if (< (Class|FindSessionsCallbackProxy|GetCurrentPlayers _array_element) (Class|FindSessionsCallbackProxy|GetMaxPlayers _array_element))
      (if (> (Class|FindSessionsCallbackProxy|GetCurrentPlayers _array_element) (LocalVariables|GetLocalMaxPlayers))
        (LocalVariables|SetLocalMaxPlayers (Class|FindSessionsCallbackProxy|GetCurrentPlayers _array_element))
        (LocalVariables|SetLocalSession _array_element)
        (LocalVariables|SetLocalGotSession true))))
  (return (LocalVariables|GetLocalSession) (LocalVariables|GetLocalGotSession)))

(fn ReleaseSpirit
  (bind _asmmocharacter (Utilities|Casting|CastToMMOCharacter (Pawn|GetControlledPawn)))
  (Variables|Default|SetLocalChar _asmmocharacter)
  (Class|MMOCharacter|SetTargetActor _asmmocharacter)
  (Networking|SwitchHasAuthority
    (:Authority
      (bind _outactors (Actor|GetAllActorsOfClass "/Game/Blueprints/Spirit/BP_Shrine.BP_Shrine_C"))
      (bind _array_element (Utilities|Array|ForEachLoopwithBreak _outactors)
        (:LoopBody
          (Utilities|IsValid _array_element
            (:Is%20Valid
              (Class|MShrine|ReleaseSpirit _array_element self (Variables|Default|GetLocalChar))
              (return))))))
    (:Remote
      (CallFunction|ServerReleaseSpirit))))

(fn ReturntoLife
  (Networking|SwitchHasAuthority
    (:Authority
      (bind _asbp_mspirit (Utilities|Casting|CastToBP_MSpirit (Pawn|GetControlledPawn)))
      (bind _corpse (Variables|/Game/Blueprints/Spirit/BP_MSpirit.BP_MSpirit_C|GetCorpse _asbp_mspirit)
        (:then
          (bind _asbp_mmocharacter (Utilities|Casting|CastToBP_MMOCharacter _corpse))
          (Default|ReturntoLife _asbp_mmocharacter self _asbp_mspirit))
        (:else)))
    (:Remote
      (CallFunction|ServerReturntoLife))))