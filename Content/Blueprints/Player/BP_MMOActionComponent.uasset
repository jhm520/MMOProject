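; MMO character action component that runs a character's abilities: requests, validation, instant or timed casts, cooldowns and auto-casting.
; Requests run on authority, and DoAction checks target, death, range and cooldown before applying the action or starting a cast.
; Applied actions spawn BP_ActionInstance actors, which double as cooldown records until they expire on tick.
; Tick also re-fires the auto-cast list on the current target and advances or cancels the active cast.
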(event Custom|OnLeftCombat
  (Utilities|Array|Clear (Variables|Default|GetAutoCastList)))

(event Custom|SetupActionMap
  (bind _asmmocharacter (Utilities|Casting|CastToMMOCharacter (Components|GetOwner)))
  (for _array_element (Variables|/Script/MMOProject.MMOCharacter|GetActionList _asmmocharacter)
    (if (.ReturnValue (Class|MHelperLibrary|GetActionwithName _array_element 0))
      (Utilities|Map|Add (Variables|Default|GetActionMap) _array_element (.OutActionData (Class|MHelperLibrary|GetActionwithName _array_element 0))))))

(event Custom|StartCasting
  (params (InAction :type Action%20Struct%20Structure) (TargetActor :type Actor%20Object%20Reference) (TargetLocation :type Vector))
  (Utilities|HasAuthority
    (:true
      (if (Utilities|Name|Equal(Name) (Variables|Default|GetCastingSpell) "None")
        (Variables|Default|SetCastingSpell (.ActionName (Utilities|Struct|BreakActionStruct InAction)))
        (Variables|Default|SetCastStartTime (Utilities|Time|GetTimeSeconds))
        (Variables|Default|SetCastTargetLocation TargetLocation)
        (Variables|Default|SetCastTarget TargetActor)))))

(event Custom|OnCanceledCasting
  (params (InAction :type Action%20Struct%20Structure) (Target :type Actor%20Object%20Reference) (TargetLocation :type Vector))
  (Utilities|HasAuthority
    (:true
      (Variables|Default|SetCastingSpell "None")
      (Variables|Default|SetCastStartTime 0.0)
      (Variables|Default|SetCastTarget 0)
      (Variables|Default|SetCastTargetLocation "0, 0, 0")
      (Variables|Default|SetCastProgress 0.0))))

(event Custom|OnFinishedCasting
  (params (InAction :type Action%20Struct%20Structure) (Target :type Actor%20Object%20Reference) (TargetLocation :type Vector))
  (Utilities|HasAuthority
    (:true
      (CallFunction|ApplyAction InAction Target TargetLocation)
      (Variables|Default|SetCastingSpell "None")
      (Variables|Default|SetCastStartTime 0.0)
      (Variables|Default|SetCastTarget 0)
      (Variables|Default|SetCastTargetLocation "0, 0, 0")
      (Variables|Default|SetCastProgress 0.0))))

(event EventTick
  (params (DeltaSeconds :type Float%20%28single-precision%29))
  (|CallParentFunction DeltaSeconds)
  (CallFunction|TickCooldowns DeltaSeconds)
  (CallFunction|TickActions DeltaSeconds)
  (CallFunction|TickCasting DeltaSeconds))

(event EventBeginPlay
  (|CallParentFunction)
  (CallFunction|SetupActionMap))

(event EventRequestDoAction
  (params (InActionName :type Name :default "None") (TargetActor :type Actor%20Object%20Reference) (TargetLocation :type Vector :default "0, 0, 0"))
  (bind _self self)
  (bind (_outactiondata _returnvalue) (Class|MHelperLibrary|GetActionwithName InActionName _self))
  (|CallParentFunction InActionName TargetActor TargetLocation)
  (Utilities|HasAuthority
    (:true
      (if _returnvalue
        (CallFunction|DoAction _outactiondata TargetActor TargetLocation)))))

(event Custom|ClientOnActionStartedCooldown
  (params (ActionName :type Name) (ActionNotify :type Character%20Action%20Notify%20Structure)))

(event Custom|ClientOnActionFinishedCooldown
  (params (ActionName :type Name) (ActionNotify :type Character%20Action%20Notify%20Structure)))

(event Custom|StartCooldown
  (params (ActionInstance :type BP%20Action%20Instance%20Object%20Reference))
  (Utilities|Map|Add (Variables|Default|GetActionInstanceMap) (.ActionName (Utilities|Struct|BreakActionStruct (.Action (Utilities|Struct|BreakCharacterActionNotify (Variables|/Game/Blueprints/Actions/BP_ActionInstance.BP_ActionInstance_C|GetActionNotify ActionInstance))))) ActionInstance))

(event Custom|LocalOnActionStarted
  (params (InActionInstance :type BP%20Action%20Instance%20Object%20Reference))
  (Utilities|Map|Add (Variables|Default|GetActionInstanceMap) (.actionname (.action (Variables|/Game/Blueprints/Actions/BP_ActionInstance.BP_ActionInstance_C|GetActionNotify InActionInstance))) InActionInstance))

(event Custom|LocalOnActionFinished
  (params (InActionInstance :type BP%20Action%20Instance%20Object%20Reference))
  (Utilities|Map|Remove (Variables|Default|GetActionInstanceMap) (.actionname (.action (Variables|/Game/Blueprints/Actions/BP_ActionInstance.BP_ActionInstance_C|GetActionNotify InActionInstance)))))

(event EventOnActionFailure
  (params (InActionStruct :type Action%20Struct%20Structure%20%28by%20ref%29) (FailureReason :type EActionFailureType%20Enum :default "Cooldown") (bNotifyServer :type Boolean))
  (bind _actionname (Utilities|Struct|BreakActionStruct InActionStruct))
  (bind _returnvalue (Utilities|String|ToString(Name) _actionname))
  (|CallParentFunction InActionStruct FailureReason bNotifyServer)
  (switch Utilities|FlowControl|Switch|SwitchonEActionFailureType FailureReason
    (:Cooldown
      (Development|PrintString (Utilities|String|Append _returnvalue " spell was on cooldown")))
    (:NoTarget
      (Utilities|Array|RemoveItem (Variables|Default|GetAutoCastList) _actionname)
      (Development|PrintString (Utilities|String|Append _returnvalue " spell had no target")))
    (:InvalidTarget
      (Utilities|Array|RemoveItem (Variables|Default|GetAutoCastList) _actionname)
      (Development|PrintString (Utilities|String|Append _returnvalue " had invalid target")))
    (:OutOfRange
      (Development|PrintString (Utilities|String|Append _returnvalue " was out of range")))))

(event EventOnActionSuccess
  (params (InActionNotify :type Character%20Action%20Notify%20Structure%20%28by%20ref%29))
  (bind (_action _instigator _targetactor) (Utilities|Struct|BreakCharacterActionNotify InActionNotify))
  (Development|PrintString (Utilities|String|Append (Utilities|GetDisplayName _instigator) "did action " (Utilities|String|ToString(Name) (.ActionName (Utilities|Struct|BreakActionStruct _action))) " to " (Utilities|GetDisplayName _targetactor))))

(fn TickCooldowns
  (params (DeltaTime :type Float%20%28single-precision%29))
  (Utilities|FlowControl|Sequence
    (:then_0
      (bind _keys (Utilities|Map|Keys (Variables|Default|GetActionInstanceMap)))
      (for _array_element _keys
        (if (.ReturnValue (Utilities|Map|Find (Variables|Default|GetActionInstanceMap) _array_element))
          (if (> (- (Utilities|Time|GetTimeSeconds) (.TimeOfCast (Utilities|Struct|BreakCharacterActionNotify (Variables|/Game/Blueprints/Actions/BP_ActionInstance.BP_ActionInstance_C|GetActionNotify (.Value (Utilities|Map|Find (Variables|Default|GetActionInstanceMap) _array_element)))))) (.CooldownTime (Utilities|Struct|BreakActionStruct (.Action (Utilities|Struct|BreakCharacterActionNotify (Variables|/Game/Blueprints/Actions/BP_ActionInstance.BP_ActionInstance_C|GetActionNotify (.Value (Utilities|Map|Find (Variables|Default|GetActionInstanceMap) _array_element))))))))
            (Utilities|Array|Add (LocalVariables|GetDoneCooldowns) (.ActionName (Utilities|Struct|BreakActionStruct (.Action (Utilities|Struct|BreakCharacterActionNotify (Variables|/Game/Blueprints/Actions/BP_ActionInstance.BP_ActionInstance_C|GetActionNotify (.Value (Utilities|Map|Find (Variables|Default|GetActionInstanceMap) _array_element))))))))))))
    (:then_1
      (for _array_element_2 (LocalVariables|GetDoneCooldowns)
        (CallFunction|EndCooldown _array_element_2)))))

(fn EndCooldown
  (params (InCooldownName :type Name))
  (bind _actioninstancemap (Variables|Default|GetActionInstanceMap))
  (bind _actioninstancemap_2 (Variables|Default|GetActionInstanceMap))
  (bind (_value _returnvalue) (Utilities|Map|Find _actioninstancemap_2 InCooldownName))
  (if _returnvalue
    (LocalVariables|SetLocalActionNotify (Variables|/Game/Blueprints/Actions/BP_ActionInstance.BP_ActionInstance_C|GetActionNotify _value))
    (Actor|DestroyActor (.Value (Utilities|Map|Find _actioninstancemap InCooldownName)))
    (Utilities|Map|Remove _actioninstancemap InCooldownName)))

(fn ApplyAction
  (params (InAction :type Action%20Struct%20Structure) (InActor :type Actor%20Object%20Reference) (InTargetLocation :type Vector))
  (bind _returnvalue (Components|GetOwner))
  (bind _aspawn (Utilities|Casting|CastToPawn _returnvalue))
  (LocalVariables|SetLocalTargetLocation InTargetLocation)
  (LocalVariables|SetLocalTargetActor InActor)
  (LocalVariables|SetLocalActionNotify (Utilities|Struct|MakeCharacterActionNotify InAction (Components|GetOwner) InActor InTargetLocation (Utilities|Time|GetTimeSeconds)))
  (Utilities|IsValid InActor
    (:Is%20Valid
      (if (CallFunction|IsValidTarget (.TargetActor (Utilities|Struct|BreakCharacterActionNotify (LocalVariables|GetLocalActionNotify))) (LocalVariables|GetLocalActionNotify))
        (bind _returnvalue_2 (Game|SpawnActorfromClass "/Game/Blueprints/Actions/BP_ActionInstance.BP_ActionInstance_C" (Math|Transform|MakeTransform "0, 0, 0") "AlwaysSpawn" (Pawn|GetController _aspawn) (LocalVariables|GetLocalActionNotify) _aspawn))
        (CallFunction|StartCooldown _returnvalue_2)
        (else
          (Class|MMOActionComponent|OnActionFailure (.Action (Utilities|Struct|BreakCharacterActionNotify (LocalVariables|GetLocalActionNotify))) "InvalidTarget" true))))))

(fn IsValidTarget
  (params (TargetActor :type Actor%20Object%20Reference) (ActionNotify :type Character%20Action%20Notify%20Structure))
  (bind _output_get (LocalVariables|SetLocalTarget TargetActor))
  (Utilities|FlowControl|Sequence
    (:then_0
      ;[1 1 1] If target is dead, return false
      (bind _asmmocharacter (Utilities|Casting|CastToMMOCharacter _output_get))
      (if (Class|MMOCharacter|IsDead _asmmocharacter)
        (return false)))
    (:then_1
      (switch Utilities|FlowControl|Switch|SwitchonEActionTargetType (.TargetType (Utilities|Struct|BreakActionStruct (.Action (Utilities|Struct|BreakCharacterActionNotify ActionNotify))))
        (:NoTarget
          _)
        (:Target
          (return (Utilities|IsValid (LocalVariables|GetLocalTarget))))
        (:TargetSelf
          _)
        (:TargetEnemy
          (return (and (!= (LocalVariables|GetLocalTarget) (Components|GetOwner)) (Utilities|IsValid (LocalVariables|GetLocalTarget)))))
        (:TargetAlly
          _)
        (:GroundTarget
          _))
      (return true))))

(fn DoAction
  (params (InAction :type Action%20Struct%20Structure) (InTargetActor :type Actor%20Object%20Reference) (InTargetLocation :type Vector))
  (bind _actionname (Utilities|Struct|BreakActionStruct InAction))
  (bind (_actionname_2 _targettype _casttype _casttime _usetype) (Utilities|Struct|BreakActionStruct InAction))
  (bind (_actionname_3 _targettype_2 _casttype_2 _casttime_2 _usetype_2) (Utilities|Struct|BreakActionStruct InAction))
  (bind (_bisvalid _failuretype) (CallFunction|IsActionValid InAction InTargetActor InTargetLocation))
  (bind (_actioninstance _boncooldown) (CallFunction|IsActiononCooldown _actionname_2))
  (if _bisvalid
    (Utilities|FlowControl|Sequence
      (:then_0
        (switch Utilities|FlowControl|Switch|SwitchonEActionUseType _usetype_2
          (:AutoCast
            (Utilities|Array|AddUnique (Variables|Default|GetAutoCastList) _actionname_3))))
      (:then_1
        (switch Utilities|FlowControl|Switch|SwitchonEActionCastType _casttype_2
          (:Instant
            (CallFunction|ApplyAction InAction InTargetActor InTargetLocation))
          (:Cast
            (CallFunction|StartCasting InAction InTargetActor InTargetLocation)))))
    (else
      (Utilities|FlowControl|Sequence
        (:then_0
          (switch Utilities|FlowControl|Switch|SwitchonEActionFailureType _failuretype
            (:Cooldown
              (if _boncooldown
                (switch Utilities|FlowControl|Switch|SwitchonEActionUseType _usetype :!label _label
                  (:Toggle
                    _)
                  (:AutoCast
                    _))
                (bind _structout (Utilities|Struct|SetmembersinCharacterActionNotify (Variables|/Game/Blueprints/Actions/BP_ActionInstance.BP_ActionInstance_C|GetActionNotify _actioninstance) true))
                (Variables|/Game/Blueprints/Actions/BP_ActionInstance.BP_ActionInstance_C|SetActionNotify _actioninstance _structout)
                (Utilities|Array|RemoveItem (Variables|Default|GetAutoCastList) _actionname_2)))
            (:InvalidTarget
              (goto _label))
            (:LineOfSight
              (goto _label))
            (:LackPermission
              (goto _label))
            (:Disabled
              (goto _label))))
        (:then_1
          (switch Utilities|FlowControl|Switch|SwitchonEActionUseType (.UseType (Utilities|Struct|BreakActionStruct InAction))
            (:Toggle
              _)
            (:AutoCast
              _))
          (if (Utilities|Array|ContainsItem (Variables|Default|GetAutoCastList) _actionname)
            (Utilities|Array|RemoveItem (Variables|Default|GetAutoCastList) _actionname)
            (else
              (Utilities|Array|AddUnique (Variables|Default|GetAutoCastList) _actionname))))
        (:then_2
          (Class|MMOActionComponent|OnActionFailure InAction _failuretype true))))))

(fn IsActiononCooldown
  (params (InAction :type Name))
  (bind _actioninstancemap (Variables|Default|GetActionInstanceMap))
  (bind (_value _returnvalue) (Utilities|Map|Find _actioninstancemap InAction))
  (if _returnvalue
    (Utilities|IsValid _value
      (:Is%20Valid
        (return _value _returnvalue))
      (:Is%20Not%20Valid
        (return 0 false)))
    (else
      (return 0 false))))

(fn IsActioninRange
  (params (ActionName :type Name) (TargetActor :type Actor%20Object%20Reference))
  (bind _self self)
  (bind (_outactiondata _returnvalue) (Class|MHelperLibrary|GetActionwithName ActionName _self))
  (bind _castmaxrange (Utilities|Struct|BreakActionStruct _outactiondata))
  (if _returnvalue
    (if (== _castmaxrange 0.0)
      (return true)
      (else
        (return (< (Math|Vector|VectorLength (- (Transformation|GetActorLocation TargetActor) (Transformation|GetActorLocation (Components|GetOwner)))) _castmaxrange))))))

(fn TickActions
  (params (DeltaTime :type Float%20%28single-precision%29))
  (for _array_element (Variables|Default|GetAutoCastList)
    (if (.ReturnValue (Class|MHelperLibrary|GetActionwithName _array_element self))
      (bind _targetactor (Utilities|GetTargetActor)
        (:Is%20Valid
          _)
        (:Is%20Not%20Valid
          _))
      (if (.bIsValid (CallFunction|IsActionValid (.OutActionData (Class|MHelperLibrary|GetActionwithName _array_element self)) _targetactor "0, 0, 0"))
        (CallFunction|DoAction (.OutActionData (Class|MHelperLibrary|GetActionwithName _array_element self)) _targetactor "0, 0, 0")))))

(fn IsActionValid
  (params (Action :type Action%20Struct%20Structure) (TargetActor :type Actor%20Object%20Reference) (Location :type Vector))
  (bind (_actionname _targettype) (Utilities|Struct|BreakActionStruct Action))
  (Utilities|FlowControl|Sequence
    (:then_0
      (bind _asmmocharacter (Utilities|Casting|CastToMMOCharacter TargetActor))
      (if (Class|MMOCharacter|IsDead _asmmocharacter)
        (return false "InvalidTarget")))
    (:then_1
      (bind _asmmocharacter_2 (Utilities|Casting|CastToMMOCharacter (Components|GetOwner)))
      (if (Class|MMOCharacter|IsDead _asmmocharacter_2)
        (return false "Disabled")))
    (:then_2
      (if (.bOnCooldown (CallFunction|IsActiononCooldown _actionname))
        (return false "Cooldown")))
    (:then_3
      (switch Utilities|FlowControl|Switch|SwitchonEActionTargetType _targettype
        (:NoTarget
          _)
        (:Target
          (bind _targetactor (Utilities|GetTargetActor :!label _label)
            (:Is%20Valid
              (if (CallFunction|IsActioninRange _actionname _targetactor) :!label _label_2
                (return true "OutOfRange")
                (else
                  (return false "OutOfRange"))))
            (:Is%20Not%20Valid
              (return true "NoTarget"))))
        (:TargetSelf
          _)
        (:TargetEnemy
          (bind _targetactor_2 (Utilities|GetTargetActor)
            (:Is%20Valid
              (if (== _targetactor_2 (Components|GetOwner))
                (return false "InvalidTarget")
                (else
                  (goto _label_2))))
            (:Is%20Not%20Valid
              (return false "NoTarget"))))
        (:TargetAlly
          (goto _label))
        (:GroundTarget
          _))
      (return true "Cooldown"))))

(fn TickCasting
  (params (DeltaTime :type Float%20%28single-precision%29))
  (bind _returnvalue (Utilities|Time|GetTimeSeconds))
  (bind _self self)
  (bind _castingspell (Variables|Default|GetCastingSpell))
  (bind _caststarttime (Variables|Default|GetCastStartTime))
  (bind (_outactiondata _returnvalue_2) (Class|MHelperLibrary|GetActionwithName _castingspell _self))
  (bind _returnvalue_3 (- _returnvalue _caststarttime))
  (bind _casttime (Utilities|Struct|BreakActionStruct _outactiondata))
  (Utilities|HasAuthority
    (:true
      (if (Utilities|Name|NotEqual(Name) (Variables|Default|GetCastingSpell) "None")
        (bind _asmmocharacter (Utilities|GetCharacter)
          (:then
            (if _returnvalue_2
              (if (Class|MMOCharacter|IsDead _asmmocharacter)
                (CallFunction|OnCanceledCasting _outactiondata (Variables|Default|GetCastTarget) (Variables|Default|GetCastTargetLocation))
                (else
                  (Variables|Default|SetCastProgress (/ _returnvalue_3 _casttime))
                  (if (>= _returnvalue_3 _casttime)
                    (CallFunction|OnFinishedCasting _outactiondata (Variables|Default|GetCastTarget) (Variables|Default|GetCastTargetLocation))))))))))))

(fn IsActionAutoCasting
  (params (InActionName :type Name))
  (return (Utilities|Array|ContainsItem (Variables|Default|GetAutoCastList) InActionName)))