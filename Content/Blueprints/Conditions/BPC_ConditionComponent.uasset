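; Actor component that tracks timed conditions on its owner, with special handling for taunts, on authority only.
; Conditions resolved from an action notify are applied as timestamped records, and a taunt also stores its instigator as TauntActor.
; Tick collects expired indices, then removes them in a second pass.
; Ending a taunt messages the owner and clears TauntActor; HasTauntCondition reports the taunt state and actor.
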(event EventBeginPlay)

(event EventTick
  (params (DeltaSeconds :type Float%20%28single-precision%29))
  (CallFunction|TickConditions DeltaSeconds))

(fn ApplyCondition
  (params (InCondition :type Condition%20Struct%20Structure) (Instigator :type Actor%20Object%20Reference))
  (Utilities|HasAuthority
    (:true
      (LocalVariables|SetLocalInstigator Instigator)
      (bind _output_get (LocalVariables|SetLocalCondition InCondition))
      (Utilities|Array|Add (Variables|Default|GetCurrentConditions) (Utilities|Struct|MakeConditionNotify (Components|GetOwner) Instigator (Utilities|Time|GetTimeSeconds) (LocalVariables|GetLocalCondition)))
      (if (CallFunction|IsTauntCondition (LocalVariables|GetLocalCondition))
        (Variables|Default|SetTauntActor (LocalVariables|GetLocalInstigator))))))

(fn ApplyConditionsfromAction
  (params (Notify :type Character%20Action%20Notify%20Structure))
  (bind (_action _instigator) (Utilities|Struct|BreakCharacterActionNotify Notify))
  (for _array_element (.TargetConditions (Utilities|Struct|BreakActionStruct _action))
    (Development|PrintString (Utilities|String|ToString(Name) _array_element))
    (if (.ReturnValue (Class|MActionDataAsset|GetConditionStruct _array_element))
      (CallFunction|ApplyCondition (.OutConditionStruct (Class|MActionDataAsset|GetConditionStruct _array_element)) _instigator))))

(fn TickConditions
  (params (DeltaTime :type Float%20%28single-precision%29))
  (bind _currentconditions (Variables|Default|GetCurrentConditions))
  (Utilities|HasAuthority
    (:true
      (Utilities|FlowControl|Sequence
        (:then_0
          (for (_array_element _array_index) (Variables|Default|GetCurrentConditions)
            (Utilities|FlowControl|Sequence
              (:then_0
                ;[1 1 1] Mark conditions for completion
                (if (>= (- (Utilities|Time|GetTimeSeconds) (.ConditionStartTime (Utilities|Struct|BreakConditionNotify _array_element))) (.ConditionTimeLength (Utilities|Struct|BreakConditionStruct (.Condition (Utilities|Struct|BreakConditionNotify _array_element)))))
                  (Utilities|Array|Add (LocalVariables|GetCompleteConditionIndices) _array_index))))))
        (:then_1
          ;[1 1 1] End complete conditions
          (for _array_element_2 (LocalVariables|GetCompleteConditionIndices)
            (LocalVariables|SetLocalCondition (Utilities|Array|Get(acopy) _currentconditions _array_element_2))
            (Utilities|Array|RemoveIndex _currentconditions _array_element_2)
            (CallFunction|EndCondition (LocalVariables|GetLocalCondition))))))))

(fn IsTauntCondition
  (params (IsTauntCondition :type Condition%20Struct%20Structure))
  (for _array_element (.ConditionEffects (Utilities|Struct|BreakConditionStruct IsTauntCondition))
    (switch Utilities|FlowControl|Switch|SwitchonEConditionEffectType (.EffectType (Utilities|Struct|BreakConditionEffectStruct _array_element))
      (:Taunt
        (return true))))
  (return false))

(fn HasTauntCondition
  (for _array_element (Variables|Default|GetCurrentConditions)
    (if (CallFunction|IsTauntCondition (.Condition (Utilities|Struct|BreakConditionNotify _array_element)))
      (return true (Variables|Default|GetTauntActor))))
  (return false 0))

(fn EndCondition
  (params (InConditionNotify :type Condition%20Notify%20Structure))
  (Utilities|FlowControl|Sequence
    (:then_0
      (if (CallFunction|IsTauntCondition (.Condition (Utilities|Struct|BreakConditionNotify InConditionNotify)))
        (Class|BPIActionInterface|OnConditionEnded(Message) (Components|GetOwner) InConditionNotify)
        (Variables|Default|SetTauntActor 0)))))