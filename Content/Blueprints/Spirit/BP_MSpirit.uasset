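; BP_MSpirit is the spirit pawn a player controls after death in an MMO, linked to the corpse left behind.
; On BeginPlay it copies the corpse's skeletal mesh, anim class and camera rotation, then notifies the owning controller's HUD that the spirit was released.
; Each tick it compares its distance to the corpse against ReviveDistance and reports the result to player 0's HUD widget.
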(event EventBeginPlay
  (bind _mesh (Variables|Character|GetMesh))
  (|CallParentFunction)
  (Utilities|FlowControl|Sequence
    (:then_0
      (bind _corpse (Variables|Default|GetCorpse)
        (:then
          (Class|SkinnedMeshComponent|SetSkeletalMesh _mesh (Variables|/Script/Engine.SkinnedMeshComponent|GetSkeletalMesh (Variables|/Script/Engine.Character|GetMesh _corpse)) true)
          (Class|SkeletalMeshComponent|SetAnimClass _mesh (Utilities|GetClass (Components|SkeletalMesh|GetAnimInstance (Variables|/Script/Engine.Character|GetMesh _corpse))))
          (Transformation|SetRelativeRotation (Variables|Default|GetCameraRoot) (Variables|/Script/Engine.SceneComponent|GetRelativeRotation (Variables|/Script/MMOProject.MMOCharacter|GetCameraRoot _corpse)) false false))
        (:else)))
    (:then_1
      (bind _asbp_mmoplayer_controller (Utilities|Casting|CastToBP_MMOPlayerController (Components|GetOwner)))
      (bind _asbp_mmohud (Utilities|Casting|CastToBP_MMOHUD (HUD|GetHUD _asbp_mmoplayer_controller)))
      (Default|OnReleasedSpirit (Variables|/Game/Blueprints/UI/BP_MMOHUD.BP_MMOHUD_C|GetMMOHudWidget _asbp_mmohud)))))

(event Collision|EventActorBeginOverlap
  (params (OtherActor :type Actor%20Object%20Reference)))

(event EventTick
  (params (DeltaSeconds :type Float%20%28single-precision%29))
  (|CallParentFunction DeltaSeconds)
  (CallFunction|TickSpirit))

(fn ConstructionScript)

(fn TickSpirit
  (bind _corpse (Variables|Default|GetCorpse)
    (:then
      (if (< (Math|Vector|VectorLength (- (Transformation|GetActorLocation _corpse) (Transformation|GetActorLocation))) (Variables|Default|GetReviveDistance))
        (CallFunction|SetClosetoCorpse true)
        (else
          (CallFunction|SetClosetoCorpse false))))
    (:else)))

(fn SetClosetoCorpse
  (params (bClose :type Boolean))
  (bind _asbp_mmoplayer_controller (Utilities|Casting|CastToBP_MMOPlayerController (Game|GetPlayerController 0)))
  (bind _asbp_mmohud (Utilities|Casting|CastToBP_MMOHUD (HUD|GetHUD _asbp_mmoplayer_controller)))
  (Default|OnClosetoCorpse (Variables|/Game/Blueprints/UI/BP_MMOHUD.BP_MMOHUD_C|GetMMOHudWidget _asbp_mmohud) bClose))