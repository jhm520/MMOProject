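; BP_Mob is a mob Blueprint that handles damage, death and proximity tracking.
; Damage is ignored during an aggro reset; otherwise it lowers Health, clamped at zero, and fires OnHealthChanged.
; That calls the parent version, then checks for death, which prints a message and sets a short life span for delayed removal.
; A Sphere component maintains OverlappingActors on the authority only, adding and removing actors on overlap.
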(event OnComponentBeginOverlap(Sphere)
  (params (OverlappedComponent :type Primitive%20Component%20Object%20Reference) (OtherActor :type Actor%20Object%20Reference) (OtherComp :type Primitive%20Component%20Object%20Reference) (OtherBodyIndex :type Integer) (bFromSweep :type Boolean) (SweepResult :type Hit%20Result%20Structure%20%28by%20ref%29))
  (Networking|SwitchHasAuthority
    (:Authority
      (Utilities|Array|Add (Variables|Default|GetOverlappingActors) OtherActor))))

(event OnComponentEndOverlap(Sphere)
  (params (OverlappedComponent :type Primitive%20Component%20Object%20Reference) (OtherActor :type Actor%20Object%20Reference) (OtherComp :type Primitive%20Component%20Object%20Reference) (OtherBodyIndex :type Integer))
  (Networking|SwitchHasAuthority
    (:Authority
      (Utilities|Array|RemoveItem (Variables|Default|GetOverlappingActors) OtherActor))))

(event Custom|OnDeath
  (Actor|SetLifeSpan 1e+01)
  (Development|PrintString (Utilities|String|Append (Utilities|GetDisplayName self) " has died")))

(event EventBeginPlay)

(event Collision|EventActorBeginOverlap
  (params (OtherActor :type Actor%20Object%20Reference)))

(event EventTick
  (params (DeltaSeconds :type Float%20%28single-precision%29)))

(event Game|Damage|EventAnyDamage
  (params (Damage :type Float%20%28single-precision%29) (DamageType :type Damage%20Type%20Object%20Reference) (InstigatedBy :type Controller%20Object%20Reference) (DamageCauser :type Actor%20Object%20Reference))
  ;[1 1 1] Can't damage this mob if it's resetting aggro
  (if (not (Variables|Default|GetbAggroReset))
    (Variables|Default|SetHealth (Math|Float|Max(Float) (- (Variables|Default|GetHealth) Damage) 0.0))
    (Class|MMOCharacter|OnHealthChanged)))

(event EventOnHealthChanged
  (|CallParentFunction)
  (if (Class|MMOCharacter|IsDead)
    (CallFunction|OnDeath)))

(fn ConstructionScript)