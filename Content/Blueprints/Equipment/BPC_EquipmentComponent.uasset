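; Equipment component that tracks which named items its owner has equipped and replicates that list.
; TryEquip adds or removes a name in ReppedEquipment on the authority, and otherwise forwards the request through ServerEquip.
; Both the authority change and the RepNotify call OnEquipmentChanged, which rebuilds EquipmentCategoryMap from equipment struct lookups.
; The map is keyed by category, so it holds one item per category, with later entries overwriting earlier ones.
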(event Custom|TryEquip
  (params (InEquipmentName :type Name) (bEquip :type Boolean))
  (Utilities|HasAuthority
    (:true
      (Utilities|FlowControl|Sequence
        (:then_0
          (if bEquip
            (Utilities|Array|Add (Variables|Default|GetReppedEquipment) InEquipmentName)
            (else
              (Utilities|Array|RemoveItem (Variables|Default|GetReppedEquipment) InEquipmentName))))
        (:then_1
          (CallFunction|OnEquipmentChanged))))
    (:false
      (CallFunction|ServerEquip InEquipmentName bEquip))))

(event Custom|ServerEquip
  (params (InEquipmentName :type Name) (bEquip :type Boolean))
  (CallFunction|TryEquip InEquipmentName bEquip))

(event EventBeginPlay)

(event EventTick
  (params (DeltaSeconds :type Float%20%28single-precision%29)))

(fn OnRepReppedEquipment
  (CallFunction|OnEquipmentChanged))

(fn OnEquipmentChanged
  (Utilities|Map|Clear (Variables|Default|GetEquipmentCategoryMap))
  (for _array_element (Variables|Default|GetReppedEquipment)
    (if (.ReturnValue (Class|MActionDataAsset|GetEquipmentStruct _array_element))
      (Utilities|Map|Add (Variables|Default|GetEquipmentCategoryMap) (.EquipmentCategoryName (Utilities|Struct|BreakEquipmentStruct (.OutEquipmentStruct (Class|MActionDataAsset|GetEquipmentStruct _array_element)))) (.OutEquipmentStruct (Class|MActionDataAsset|GetEquipmentStruct _array_element))))))