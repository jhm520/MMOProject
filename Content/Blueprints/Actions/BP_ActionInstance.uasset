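; BP_ActionInstance is the actor representing one cast of an MMO action, applying its damage to the target actor.
; On authority, Instant spells apply damage at BeginPlay, while Projectile spells home toward the target each tick and apply it on proximity.
; It reports start, success and finish to the instigator's BP_MMOActionComponent.
; Tick tracks time since cast, and projectiles destroy themselves after impact only if the action is off cooldown.
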(event EventBeginPlay
  (|CallParentFunction)
  (Utilities|FlowControl|Sequence
    (:then_0
      (Networking|SwitchHasAuthority
        (:Authority
          (switch Utilities|FlowControl|Switch|SwitchonEActionSpellType (.SpellType (Utilities|Struct|BreakActionStruct (.Action (Utilities|Struct|BreakCharacterActionNotify (Variables|Default|GetActionNotify)))))
            (:Instant
              (CallFunction|ApplyEffects))))))
    (:then_1
      (bind _asmmocharacter (Utilities|Casting|CastToMMOCharacter (Game|GetInstigator)))
      (Utilities|FlowControl|Sequence
        (:then_0
          (Default|LocalonActionStarted (Actor|GetComponentbyClass _asmmocharacter "/Game/Blueprints/Player/BP_MMOActionComponent.BP_MMOActionComponent_C") self))
        (:then_1
          (Class|MMOActionComponent|OnActionSuccess (Actor|GetComponentbyClass _asmmocharacter "/Game/Blueprints/Player/BP_MMOActionComponent.BP_MMOActionComponent_C") (Variables|Default|GetActionNotify)))))))

(event Collision|EventActorBeginOverlap
  (params (OtherActor :type Actor%20Object%20Reference)))

(event EventTick
  (params (DeltaSeconds :type Float%20%28single-precision%29))
  (|CallParentFunction DeltaSeconds)
  (Networking|SwitchHasAuthority
    (:Authority
      (Variables|Default|SetCurrentCooldownTime (- (Utilities|Time|GetTimeSeconds) (.timeofcast (Variables|Default|GetActionNotify))))
      (CallFunction|TickProjectile DeltaSeconds))))

(event EventDestroyed
  (Utilities|FlowControl|Sequence
    (:then_0
      (bind _asmmocharacter (Utilities|Casting|CastToMMOCharacter (Game|GetInstigator)))
      (Default|LocalonActionFinished (Actor|GetComponentbyClass _asmmocharacter "/Game/Blueprints/Player/BP_MMOActionComponent.BP_MMOActionComponent_C") self))
    (:then_1
      (|CallParentFunction))))

(fn ConstructionScript)

(fn OnRepAction)

(fn TickProjectile
  (params (DeltaSeconds :type Float%20%28single-precision%29))
  (bind _returnvalue (Transformation|GetActorLocation))
  (bind _actionnotify (Variables|Default|GetActionNotify))
  (bind (_action _instigator _targetactor) (Utilities|Struct|BreakCharacterActionNotify _actionnotify))
  (bind (_actionname _targettype _casttype _spelltype _projectilespeed) (Utilities|Struct|BreakActionStruct _action))
  (bind _returnvalue_2 (Transformation|GetActorLocation _targetactor))
  (bind _returnvalue_3 (- _returnvalue_2 _returnvalue))
  (if (not (Variables|Default|GetbAppliedEffects))
    (switch Utilities|FlowControl|Switch|SwitchonEActionSpellType _spelltype
      (:Instant
        (return))
      (:Projectile
        (Utilities|FlowControl|Sequence
          (:then_0
            (Utilities|IsValid _targetactor
              (:Is%20Valid
                (Transformation|SetActorLocation (+ (Transformation|GetActorLocation) (* (* (Math|Vector|Normalize _returnvalue_3) _projectilespeed) DeltaSeconds)) false false))))
          (:then_1
            (if (< (Math|Vector|VectorLength _returnvalue_3) 1e+02)
              (Networking|SwitchHasAuthority
                (:Authority
                  (CallFunction|ApplyEffects))))))))))

(fn ApplyEffects
  (bind _actionnotify (Variables|Default|GetActionNotify))
  (bind _actionnotify_2 (Variables|Default|GetActionNotify))
  (bind _action (Utilities|Struct|BreakCharacterActionNotify _actionnotify_2))
  (bind (_actionname _targettype _casttype _spelltype _projectilespeed _casttime _usetype _damage _cooldowntime _castmaxrange _damagetype) (Utilities|Struct|BreakActionStruct _action))
  (Game|Damage|ApplyDamage (.targetactor _actionnotify) _damage (.AsController (Utilities|Casting|CastToController (Components|GetOwner))) (.instigator _actionnotify) _damagetype)
  (Variables|Default|SetbAppliedEffects true)
  (switch Utilities|FlowControl|Switch|SwitchonEActionSpellType (.SpellType (Utilities|Struct|BreakActionStruct (.Action (Utilities|Struct|BreakCharacterActionNotify (Variables|Default|GetActionNotify)))))
    (:Projectile
      (if (not (.bOnCooldown (Default|IsActiononCooldown (CallFunction|GetActionComponent) (CallFunction|GetActionName))))
        (Actor|DestroyActor)))))

(fn GetActionComponent
  (return (Actor|GetComponentbyClass (Game|GetInstigator) "/Game/Blueprints/Player/BP_MMOActionComponent.BP_MMOActionComponent_C")))

(fn GetActionName
  (return (.ActionName (Utilities|Struct|BreakActionStruct (.Action (Utilities|Struct|BreakCharacterActionNotify (Variables|Default|GetActionNotify)))))))